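; Child character Blueprint in the Flying folder that handles axis input for moving on three axes and turning.
; Forward, right and up inputs scale the TopDownCameraComponent's matching vectors by MovementMagnitude and feed CharacterMovement's AddInputVector.
; Each passes only one world component (X, Y or Z respectively), discarding the rest of the camera direction.
; LookRight yaws the actor by RotationMagnitude times the axis value, without delta-time scaling.
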(event `InputAxis|LookRight`
  (params (AxisValue :type "Float (single-precision)"))
  (`self.K2_AddActorWorldRotation` (`KismetMathLibrary.MakeRotator` 0.0 0.0 (* (`self.RotationMagnitude`) AxisValue))))

(event `InputAxis|MoveForward`
  (params (AxisValue :type "Float (single-precision)"))
  (`PawnMovementComponent.AddInputVector` (`self.CharacterMovement`) (`KismetMathLibrary.MakeVector` (.x (* (* (`SceneComponent.GetForwardVector` (`self.TopDownCameraComponent`)) (`self.MovementMagnitude`)) AxisValue))) false))

(event `InputAxis|MoveRight`
  (params (AxisValue :type "Float (single-precision)"))
  (`PawnMovementComponent.AddInputVector` (`self.CharacterMovement`) (`KismetMathLibrary.MakeVector` 0.0 (.y (* (* (`SceneComponent.GetRightVector` (`self.TopDownCameraComponent`)) (`self.MovementMagnitude`)) AxisValue))) false))

(event `InputAxis|MoveUp`
  (params (AxisValue :type "Float (single-precision)"))
  (`PawnMovementComponent.AddInputVector` (`self.CharacterMovement`) (`KismetMathLibrary.MakeVector` 0.0 0.0 (.z (* (* (`SceneComponent.GetUpVector` (`self.TopDownCameraComponent`)) (`self.MovementMagnitude`)) AxisValue))) false))

(fn `UserConstructionScript`
  (`parent.UserConstructionScript`))