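; Flying player character that moves with a boom-mounted camera and tracks which compass direction it faces.
; Movement axes scale camera direction vectors by Acceleration but pass only one world component each to CharacterMovement, and vertical input stops above a height ceiling.
; LookRight yaws the camera boom and ZoomFactor changes its arm length, while LookUp is empty.
; Tick sets PlayerDir from 2D dot products of mesh forward against MapObject's axes.
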(event `InputAxis|LookUp`
  (params (AxisValue :type "Float (single-precision)")))

(event `InputAxis|LookRight`
  (params (AxisValue :type "Float (single-precision)"))
  (`SceneComponent.K2_AddWorldRotation` (`self.CameraBoom`) (`KismetMathLibrary.MakeRotator` 0.0 0.0 (* (`self.TurnSpeed`) AxisValue)) false false))

(event `InputAxis|MoveForward`
  (params (AxisValue :type "Float (single-precision)"))
  (`PawnMovementComponent.AddInputVector` (`self.CharacterMovement`) (`KismetMathLibrary.MakeVector` (.x (* (* (`SceneComponent.GetForwardVector` (`self.TopDownCameraComponent`)) (`self.Acceleration`)) AxisValue))) false))

(event `InputAxis|MoveRight`
  (params (AxisValue :type "Float (single-precision)"))
  (`PawnMovementComponent.AddInputVector` (`self.CharacterMovement`) (`KismetMathLibrary.MakeVector` 0.0 (.y (* (* (`SceneComponent.GetRightVector` (`self.TopDownCameraComponent`)) (`self.Acceleration`)) AxisValue))) false))

(event `InputAxis|ZoomFactor`
  (params (AxisValue :type "Float (single-precision)"))
  (bind _cameraboom (`self.CameraBoom`))
  (bind _cameraboom_2 (`self.CameraBoom`))
  (`/Engine/EditorBlueprintResources/StandardMacros.CompareFloat` AxisValue
    (:`>`
      (set `SpringArmComponent.TargetArmLength` (+ (`SpringArmComponent.TargetArmLength` _cameraboom) (`self.SpringLegnthDelta`)) _cameraboom))
    (:`<`
      (set `SpringArmComponent.TargetArmLength` (- (`SpringArmComponent.TargetArmLength` _cameraboom_2) (`self.SpringLegnthDelta`)) _cameraboom_2))))

(event `InputAxis|MoveUp`
  (params (AxisValue :type "Float (single-precision)"))
  (`/Engine/EditorBlueprintResources/StandardMacros.CompareFloat` (.z (`self.K2_GetActorLocation`)) 70000.0
    (:`==`
      _)
    (:`<`
      _))
  (`PawnMovementComponent.AddInputVector` (`self.CharacterMovement`) (`KismetMathLibrary.MakeVector` 0.0 0.0 (.z (* (* (`SceneComponent.GetUpVector` (`self.TopDownCameraComponent`)) (`self.Acceleration`)) AxisValue))) false))

(event `self.ReceiveTick`
  (params (DeltaSeconds :type "Float (single-precision)"))
  (bind _mapobject (`self.mapObject`))
  (bind (_returnvalue_x _returnvalue_y) (`KismetMathLibrary.BreakVector` (`SceneComponent.GetForwardVector` (`self.Mesh`))))
  (bind (_returnvalue_x_2 _returnvalue_y_2) (`KismetMathLibrary.BreakVector` (`self.GetActorForwardVector` _mapobject)))
  (bind (_returnvalue_x_3 _returnvalue_y_3) (`KismetMathLibrary.BreakVector` (`self.GetActorRightVector` _mapobject)))
  (bind _returnvalue (`KismetMathLibrary.MakeVector2D` _returnvalue_x _returnvalue_y))
  (bind _returnvalue_2 (`KismetMathLibrary.MakeVector2D` _returnvalue_x_3 _returnvalue_y_3))
  (bind _returnvalue_3 (`KismetMathLibrary.DotProduct2D` _returnvalue_2 _returnvalue))
  (bind _returnvalue_4 (`KismetMathLibrary.DotProduct2D` (* _returnvalue_2 -1.0) _returnvalue))
  (`/Engine/EditorBlueprintResources/StandardMacros.IsValid` (`self.mapObject`)
    (:`Is Valid`
      (`|ExecutionSequence`
        (:`then_0`
          (`/Engine/EditorBlueprintResources/StandardMacros.CompareFloat` (`KismetMathLibrary.DotProduct2D` (`KismetMathLibrary.MakeVector2D` _returnvalue_x_2 _returnvalue_y_2) _returnvalue)
            (:`>`
              (if (`KismetMathLibrary.InRange_FloatFloat` _returnvalue_3 -0.5 0.5)
                (set `self.PlayerDir` "PD_North")
                (elif (or (`KismetMathLibrary.InRange_FloatFloat` _returnvalue_3 0.5) (`KismetMathLibrary.InRange_FloatFloat` _returnvalue_4 -1.0 -0.5))
                  (set `self.PlayerDir` "PD_East")
                  (elif (`KismetMathLibrary.InRange_FloatFloat` _returnvalue_3 -1.0 -0.5)
                    (set `self.PlayerDir` "PD_West")))))
            (:`<`
              (if (`KismetMathLibrary.InRange_FloatFloat` _returnvalue_4 -0.5 0.5)
                (set `self.PlayerDir` "PD_South")
                (elif (or (`KismetMathLibrary.InRange_FloatFloat` _returnvalue_4 0.5) (`KismetMathLibrary.InRange_FloatFloat` _returnvalue_3 -1.0 -0.5))
                  (set `self.PlayerDir` "PD_West")
                  (elif (`KismetMathLibrary.InRange_FloatFloat` _returnvalue_4 -1.0 -0.5)
                    (set `self.PlayerDir` "PD_East")))))))))))

(fn `UserConstructionScript`)