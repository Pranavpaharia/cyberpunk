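; BP_Coala_Interface2 is a UI bridge between the Coala map system, the player and the WI_Player_Coala widget.
; Its handlers push player coordinates and weather updates to the widget; map load also refreshes time, re-enables player input and removes the loading screen.
; The setup that creates both widgets, finds the player and binds these handlers is disconnected, and BeginPlay is empty, so none of it runs.
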(event `self.ReceiveBeginPlay`)

(event `NewPlayerPostion`
  (params (Lon :type "Float (double-precision)") (Lat :type "Float (double-precision)"))
  ;[1 1 1] Update Coordinates
  (bind _aswi_player_coala (cast `/ThoughtfishCoalaPlugin/Blueprints/WI_Player_Coala` (`self.UIWidget`)))
  (`/ThoughtfishCoalaPlugin/Blueprints/WI_Player_Coala.UpdateLocation` _aswi_player_coala Lon Lat))

(event `MapLoaded`
  (bind _player (`self.Player`))
  ;[1 1 1] If Map Laoded
  (bind _aswi_player_coala (cast `/ThoughtfishCoalaPlugin/Blueprints/WI_Player_Coala` (`self.UIWidget`))
    (:`then`
      (`/ThoughtfishCoalaPlugin/Blueprints/WI_Player_Coala.UpdateTime` _aswi_player_coala)
      (`/ThoughtfishCoalaPlugin/Blueprints/WI_Player_Coala.UpdateWeather` _aswi_player_coala "NewEnumerator0"))
    (:`CastFailed`
      _))
  (`/Engine/EditorBlueprintResources/StandardMacros.IsValid` _player
    (:`Is Valid`
      (`self.EnableInput` _player (`GameplayStatics.GetPlayerController` 0)))
    (:`Is Not Valid`
      _))
  ;;[0.9782 1 0.231] Remove Loading
  (`/Engine/EditorBlueprintResources/StandardMacros.IsValid` (`self.UILoading`)
    (:`Is Valid`
      (`Widget.RemoveFromParent` (`self.UILoading`)))))

(event `WeatherUpdate`
  (params (NewParam :type "/ThoughtfishCoalaPlugin/Blueprints/types/WeatherType Enum" :default "NewEnumerator0"))
  ;[1 1 1] When BP_coala received weather updates they are handled here.
  (bind _aswi_player_coala (cast `/ThoughtfishCoalaPlugin/Blueprints/WI_Player_Coala` (`self.UIWidget`)))
  (`/ThoughtfishCoalaPlugin/Blueprints/WI_Player_Coala.UpdateWeather` _aswi_player_coala NewParam))

(fn `UserConstructionScript`)